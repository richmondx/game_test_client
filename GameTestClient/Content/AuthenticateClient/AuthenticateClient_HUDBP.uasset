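; HUD Blueprint for an authentication client that shows connection state, readiness and authentication results on the AuthenticateClient_UI widget.
; Connection and run-status events set the status texts, and only the Running state marks the widget connected and enables its Authenticate button.
; Platform client messages are filtered by header, then the first block's leading character code selects whether the second block displays as an error or a token.
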(event `self.SetIsClientConnected`
  (params (is_connected :type Boolean))
  (bind _asauthenticate_client_ui (cast `/Game/AuthenticateClient/AuthenticateClient_UI` (`self.MessageResponseUI`)))
  (if is_connected
    (bind _txtconnectionstatus (`/Game/AuthenticateClient/AuthenticateClient_UI.TxtConnectionStatus` _asauthenticate_client_ui))
    (`TextBlock.SetText` _txtconnectionstatus "Connected")
    (else
      (`TextBlock.SetText` _txtconnectionstatus "Disconnected"))))

(event `self.UpdateClientRunStatus`
  (params (status :type "EClientWorkerStatus Enum" :default "EC_WORKER_UNINITIALIZED"))
  (bind _asauthenticate_client_ui (cast `/Game/AuthenticateClient/AuthenticateClient_UI` (`self.MessageResponseUI`)))
  (switch `EClientWorkerStatus` status
    (:`EC_WORKER_UNINITIALIZED`
      (bind _txtreadystatus (`/Game/AuthenticateClient/AuthenticateClient_UI.TxtReadyStatus` _asauthenticate_client_ui))
      (`TextBlock.SetText` _txtreadystatus "Not Ready" :!label _label)
      (set `/Game/AuthenticateClient/AuthenticateClient_UI.isConnected` false _asauthenticate_client_ui)
      (bind _btnauthenticate (`/Game/AuthenticateClient/AuthenticateClient_UI.BtnAuthenticate` _asauthenticate_client_ui))
      (`Widget.SetIsEnabled` _btnauthenticate false))
    (:`EC_WORKER_INITIALIZED`
      (goto _label))
    (:`EC_WORKER_STARTING`
      (goto _label))
    (:`EC_WORKER_RUNNING`
      (`TextBlock.SetText` _txtreadystatus "Ready")
      (set `/Game/AuthenticateClient/AuthenticateClient_UI.isConnected` true _asauthenticate_client_ui)
      (`Widget.SetIsEnabled` _btnauthenticate true))
    (:`EC_WORKER_STOPPING`
      (goto _label))))

(event `self.ProcessPlatformClientMessage`
  (params (message :type "PlatformClientMessage Structure"))
  (bind (_messageheader _messageblocks) (break `PlatformClientMessage` message))
  (bind _messageresponseui (`self.MessageResponseUI`))
  (bind _messagedata (break `PlatformMessageBlock` (`KismetArrayLibrary.Array_Get` _messageblocks 1)))
  (switch `int` (`KismetStringLibrary.Conv_StringToInt` (`KismetStringLibrary.Conv_ByteToString` _messageheader))
    (:`3`
      (switch `string` (`KismetStringLibrary.Conv_IntToString` (`KismetStringLibrary.GetCharacterAsNumber` (`.messageData` (break `PlatformMessageBlock` (`KismetArrayLibrary.Array_Get` _messageblocks)))))
        (:`0`
          (bind _asauthenticate_client_ui (cast `/Game/AuthenticateClient/AuthenticateClient_UI` _messageresponseui))
          (`TextBlock.SetText` (`/Game/AuthenticateClient/AuthenticateClient_UI.TxtAuthMessage` _asauthenticate_client_ui) (`KismetTextLibrary.Conv_StringToText` (`KismetStringLibrary.Concat_StrStr` "Error Message: " _messagedata))))
        (:`1`
          (bind _asauthenticate_client_ui_2 (cast `/Game/AuthenticateClient/AuthenticateClient_UI` _messageresponseui))
          (`TextBlock.SetText` (`/Game/AuthenticateClient/AuthenticateClient_UI.TxtAuthMessage` _asauthenticate_client_ui_2) (`KismetTextLibrary.Conv_StringToText` (`KismetStringLibrary.Concat_StrStr` "Authenticate Token: " _messagedata))))))))

(fn `UserConstructionScript`)