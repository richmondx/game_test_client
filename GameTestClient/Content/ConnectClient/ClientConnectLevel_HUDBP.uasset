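; HUD Blueprint for the client connection level that reports network connection and worker state on screen.
; Two events, one for the connected flag and one for run status, cast the MessageResponseUI widget to ClientConnectUI.
; They write Connected or Not Connected, or the status enum converted to text, into its status text fields.
; Construction and default lifecycle events are empty.
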(event `self.SetIsClientConnected`
  (params (is_connected :type Boolean))
  (bind _asclient_connect_ui (cast `/Game/ConnectClient/ClientConnectUI` (`self.MessageResponseUI`)))
  (if is_connected
    (bind _txtstatus (`/Game/ConnectClient/ClientConnectUI.TxtStatus` _asclient_connect_ui))
    (`TextBlock.SetText` _txtstatus "Connected")
    (else
      (`TextBlock.SetText` _txtstatus "Not Connected"))))

(event `self.UpdateClientRunStatus`
  (params (status :type "EClientWorkerStatus Enum"))
  (bind _asclient_connect_ui (cast `/Game/ConnectClient/ClientConnectUI` (`self.MessageResponseUI`)))
  (`TextBlock.SetText` (`/Game/ConnectClient/ClientConnectUI.TxtWorkerStatus` _asclient_connect_ui) (`KismetTextLibrary.Conv_StringToText` (`|GetEnumeratorNameAsString` status))))

(fn `UserConstructionScript`)