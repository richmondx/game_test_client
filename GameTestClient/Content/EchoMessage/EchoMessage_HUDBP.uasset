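; EchoMessage HUD Blueprint that relays platform client status and echo messages to an EchoMessageUI held in MessageResponseUI.
; Connection and run-status events cast that reference and update its connected and command-ready displays.
; Incoming messages switch on the header as an integer; type 1 shows the first block's data as a received echo, prefixed with a label.
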(event `self.SetIsClientConnected`
  (params (is_connected :type Boolean))
  (bind _asecho_message_ui (cast `/Game/EchoMessage/EchoMessageUI` (`self.MessageResponseUI`)))
  (`/Game/EchoMessage/EchoMessageUI.UpdateIsConnected` _asecho_message_ui is_connected))

(event `self.UpdateClientRunStatus`
  (params (status :type "EClientWorkerStatus Enum" :default "EC_WORKER_UNINITIALIZED"))
  (bind _asecho_message_ui (cast `/Game/EchoMessage/EchoMessageUI` (`self.MessageResponseUI`)))
  (`/Game/EchoMessage/EchoMessageUI.UpdateCmdReady` _asecho_message_ui status))

(event `self.ProcessPlatformClientMessage`
  (params (message :type "PlatformClientMessage Structure"))
  (bind (_messageheader _messageblocks) (break `PlatformClientMessage` message))
  (switch `int` (`KismetMathLibrary.Conv_ByteToInt` _messageheader)
    (:`1`
      (bind _asecho_message_ui (cast `/Game/EchoMessage/EchoMessageUI` (`self.MessageResponseUI`)))
      (`/Game/EchoMessage/EchoMessageUI.UpdateEchoReceive` _asecho_message_ui (`KismetStringLibrary.Concat_StrStr` "Got Msg: " (`.messageData` (break `PlatformMessageBlock` (`KismetArrayLibrary.Array_Get` _messageblocks))))))))

(fn `UserConstructionScript`)